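; BP_MyGameMode is the game mode that tracks level progress and shows the win or lose result.
; BeginPlay adds the player UI, commented as the health bar, and sets game-only input.
; Tick counts BP_Light actors and sets Exploding when that count equals PassedLights.
; AddScore triggers GameResult at a score threshold, which shows clear or game-over UI and plays a sound, whose Result parameter is always false.
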(event Custom|GameResult
  (params (Clear :type Boolean))
  (bind _returnvalue (UserInterface|CreateWidget (select Clear "/Game/UMG/ClearUI.ClearUI_C" "/Game/UMG/GameOverUI.GameOverUI_C")))
  (Variables|Default|SetClearFlag (select Clear false false))
  (UserInterface|Viewport|AddtoViewport _returnvalue 0)
  (bind _returnvalue_2 (Audio|SpawnSoundatLocation 0 "0, 0, 0" "0, 0, 0" 1.0 1.0 0.0 0 0))
  (Effects|Components|ParticleSystem|SetBoolParameter _returnvalue_2 "Result" (Variables|Default|GetClearFlag)))

(event EventBeginPlay
  (bind _returnvalue (Game|GetPlayerController 0))
  ;[1 1 1] 체력바 표시
  (bind _returnvalue_2 (UserInterface|CreateWidget "/Game/UMG/PlayerUI.PlayerUI_C"))
  (UserInterface|Viewport|AddtoViewport _returnvalue_2 0)
  (Utilities|IsValid _returnvalue
    (:Is%20Valid
      (Input|SetInputModeGameOnly _returnvalue))))

(event EventTick
  (params (DeltaSeconds :type Float%20%28single-precision%29))
  ;[1 1 1] 폭발이벤트
  (bind _outactors (Actor|GetAllActorsOfClass "/Game/BluePrints/BP_Light.BP_Light_C"))
  (bind _output_get (Variables|Default|SetNumbersOfLights (Utilities|Array|Length _outactors)))
  (if (== _output_get (Variables|Default|GetPassedLights))
    (Variables|Default|SetExploding true)))

(fn ConstructionScript)

(fn AddScore
  (bind _output_get (Variables|Default|SetTotalScore (+ (Variables|Default|GetTotalScore) 1)))
  (if (>= _output_get 5)
    (CallFunction|GameResult true)))